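; Rider-side component for broom riding that, despite its movement name, only handles getting off the mount.
; BeginPlay casts the owner to RiderCharacter and caches it along with its RidingTarget, which is not used further here.
; RidingStopped_Event detaches the rider, snaps its root to a hard-coded world transform and plays a one-shot right-side dismount animation directly on the mesh.
; Tick is empty, and nothing here binds or calls the stop event.
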(event `self.ReceiveBeginPlay`
  (bind _asrider_character (cast `RiderCharacter` (`self.GetOwner`)))
  (bind _output_get (set `self.Rider` _asrider_character))
  (set `self.Riding Target` (`RiderCharacter.RidingTarget` _output_get)))

(event `RidingStopped_Event`
  (bind _rider (`self.Rider`))
  (`Actor.K2_DetachFromActor` _rider "KeepRelative" "KeepRelative" "KeepRelative")
  (`SceneComponent.K2_SetWorldLocationAndRotation` (`Actor.RootComponent` _rider) (0.0 0.0 -10.0) (`KismetMathLibrary.MakeRotator` 0.0 90.0) false false)
  (`SkeletalMeshComponent.PlayAnimation` (`Character.Mesh` _rider) "/Game/HorseStarterKit/Animation/Dismount_Right_Rider.Dismount_Right_Rider" false))