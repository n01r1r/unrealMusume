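; A character movement component that makes its owner periodically drop bananas behind it as it moves.
; On init it runs the parent setup, then starts a looping timer with a random interval that is picked once.
; Each tick of the timer spawns a BP_Banana a short distance behind the owner's facing direction and calls DropStart on it.
; Movement itself is left to the parent component.
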(event `self.Init`
  (`parent.Init`)
  (bind _output_get (set `self.Rand Time` (`KismetMathLibrary.RandomFloatInRange` 2.0 4.0)))
  (`KismetSystemLibrary.K2_SetTimerDelegate` (delegate `DropBanana`) _output_get true))

(event `DropBanana`
  (bind _returnvalue (`self.GetOwner`))
  (bind _returnvalue_2 (`|SpawnActorFromClass` "/Game/Musume/Actor/BP_Banana.BP_Banana_C" (`KismetMathLibrary.MakeTransform` (+ (`Actor.K2_GetActorLocation` _returnvalue) (* (`Actor.GetActorForwardVector` _returnvalue) -150.0))) "Undefined" "MultiplyWithRoot" null null))
  (`/Game/Musume/Actor/BP_Banana.DropStart` _returnvalue_2))

(event `self.Movement`
  (params (DeltaTime :type "Float (single-precision)"))
  (`parent.Movement` DeltaTime))