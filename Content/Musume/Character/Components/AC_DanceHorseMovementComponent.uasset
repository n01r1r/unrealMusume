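; Horse movement component that stops its horse and hands the rider off to a dance event.
; It extends a parent movement component, leaving movement to the parent and switching its function on 15 seconds after initialization.
; The dance event zeroes the random speed range and velocity, detaches the attached RiderCharacter in place, then calls DanceEvent on that rider's AC_DanceRiderMovement component.
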(event `self.ReceiveBeginPlay`)

(event `self.ReceiveTick`
  (params (DeltaSeconds :type "Float (single-precision)")))

(event `self.Init`
  (`parent.Init`)
  (`KismetSystemLibrary.Delay` 15.0)
  (`self.ExecuteFunction` true))

(event `self.Movement`
  (params (DeltaTime :type "Float (single-precision)"))
  (`parent.Movement` DeltaTime))

(event `self.ExecuteFunction`
  (params (_IsFunctionOn :type Boolean))
  (`parent.ExecuteFunction` _IsFunctionOn)
  (if _IsFunctionOn
    (`self.Dance Event`)))

(event `Dance Event`
  (bind _owingcharacter (`self.OwingCharacter`))
  (`|ExecutionSequence`
    (:`then_0`
      (set `self.SpeedRandomValueRange` (0.0 0.0))
      (set `MovementComponent.Velocity` (0.0 0.0 0.0) (`Character.CharacterMovement` _owingcharacter)))
    (:`then_1`
      (for _array_element (`Actor.GetAttachedActors` _owingcharacter true false)
        (bind _asrider_character (cast `RiderCharacter` _array_element))
        (bind _output_get (set `self.Rider Character` _asrider_character))
        (`Actor.K2_DetachFromActor` _output_get "KeepWorld" "KeepWorld" "KeepWorld")))
    (:`then_2`
      (bind _asac_dance_rider_movement (cast `/Game/Musume/Character/Components/AC_DanceRiderMovement` (`Actor.GetComponentByClass` (`self.Rider Character`) "/Game/Musume/Character/Components/AC_DanceRiderMovement.AC_DanceRiderMovement_C")))
      (`/Game/Musume/Character/Components/AC_DanceRiderMovement.Dance Event` _asac_dance_rider_movement))))