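; Movement component for horse racer characters that defers Init and Movement to its parent class.
; Its Blueprint spline-following logic is disconnected: timer setup randomizing yaw offset and walk speed, plus per-tick steering with forward input.
; RotateToSpline aims at the spline point nearest a position projected ahead along the tangent, with CalcRotationLerpSpeed quickening interpolation as yaw error exceeds a threshold.
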(event `self.Init`
  (`parent.Init`))

(event `RotationRandomValueTimer`
  (bind (_rotationrandomvaluerange_x _rotationrandomvaluerange_y) (`KismetMathLibrary.BreakVector2D` (`self.RotationRandomValueRange`)))
  ;[1 1 1] 랜덤 Rotation 타이머
  (set `self.RotationRandomValue` (`KismetMathLibrary.RandomFloatInRange` _rotationrandomvaluerange_x _rotationrandomvaluerange_y)))

(event `SpeedRandomValueTimer`
  (bind (_speedrandomvaluerange_x _speedrandomvaluerange_y) (`KismetMathLibrary.BreakVector2D` (`self.SpeedRandomValueRange`)))
  ;[1 1 1] 랜덤 Speed 타이머
  (set `CharacterMovementComponent.MaxWalkSpeed` (`KismetMathLibrary.RandomFloatInRange` _speedrandomvaluerange_x _speedrandomvaluerange_y) (`Character.CharacterMovement` (`self.OwingCharacter`))))

(event `self.Movement`
  (params (DeltaTime :type "Float (single-precision)"))
  (`parent.Movement` DeltaTime))

(fn `CalcRotationLerpSpeed`
  (params (LookAtRotation :type "Rotator Structure"))
  (returns (LerpSpeed :type "Float (double-precision)"))
  (bind _rotationlerpspeed (`self.RotationLerpSpeed`))
  (bind _returnvalue (`KismetMathLibrary.Abs` (.yaw (`KismetMathLibrary.NormalizedDeltaRotator` LookAtRotation (`Actor.K2_GetActorRotation` (`self.OwingCharacter`))))))
  (if (<= (`self.RotationCorrectionMinYawValue`) _returnvalue)
    (return (+ _rotationlerpspeed (* _rotationlerpspeed (* (- _returnvalue (`self.RotationCorrectionMinYawValue`)) 0.1))))
    (else
      (return (`self.RotationLerpSpeed`)))))

(fn `RotateToSpline`
  (params (`Delta Time` :type "Float (double-precision)"))
  (bind _returnvalue (`Actor.K2_GetActorLocation` (`self.OwingCharacter`)))
  (bind _returnvalue_2 (`KismetMathLibrary.FindLookAtRotation` _returnvalue (`SplineComponent.FindLocationClosestToWorldLocation` (`self.TrackSplineComponent`) (+ (* (`KismetMathLibrary.Normal` (`SplineComponent.FindTangentClosestToWorldLocation` (`self.TrackSplineComponent`) _returnvalue "World")) 2000.0) _returnvalue) "World")))
  (`Actor.K2_SetActorRotation` (`self.OwingCharacter`) (`KismetMathLibrary.MakeRotator` (.roll (`KismetMathLibrary.RInterpTo` (`Actor.K2_GetActorRotation` (`self.OwingCharacter`)) (`KismetMathLibrary.MakeRotator` (.roll _returnvalue_2) (.pitch _returnvalue_2) (+ (.yaw _returnvalue_2) (`self.RotationRandomValue`))) (`local.Delta Time`) (`self.CalcRotationLerpSpeed` _returnvalue_2))) 0.0 (.yaw (`KismetMathLibrary.RInterpTo` (`Actor.K2_GetActorRotation` (`self.OwingCharacter`)) (`KismetMathLibrary.MakeRotator` (.roll _returnvalue_2) (.pitch _returnvalue_2) (+ (.yaw _returnvalue_2) (`self.RotationRandomValue`))) (`local.Delta Time`) (`self.CalcRotationLerpSpeed` _returnvalue_2)))) true))