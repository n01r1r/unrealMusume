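; Character movement component that has a rider dismount from the horse and perform a dance animation.
; DanceEvent turns and offsets the owning character, debug-prints the horse mesh's forward vector, then plays the dismount animation.
; A Delay loop polls until that finishes, then applies GetRiderRotator's rotation and starts the dance.
; GetRiderRotator's look-at math toward a point ahead of the horse is left unconnected.
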(event `self.ReceiveBeginPlay`)

(event `Dance Event`
  (bind _owingcharacter (`self.OwingCharacter`))
  (bind _owingcharacter_2 (`self.OwingCharacter`))
  (bind _mesh (`Character.Mesh` _owingcharacter))
  (`|ExecutionSequence`
    (:`then_0`
      (`Actor.K2_AddActorLocalRotation` _owingcharacter_2 (struct :`Pitch` 90.0) false false)
      (`Actor.K2_AddActorLocalOffset` _owingcharacter_2 (-130.0 0.0 80.0) false false))
    (:`then_1`
      (bind _asrider_character (cast `RiderCharacter` (`self.OwingCharacter`)))
      (bind _output_get (set `self.horse` (`RiderCharacter.RidingTarget` _asrider_character)))
      (`KismetSystemLibrary.PrintString` (`KismetStringLibrary.Conv_VectorToString` (`SceneComponent.GetForwardVector` (`Character.Mesh` _output_get)))))
    (:`then_2`
      (`SkeletalMeshComponent.PlayAnimation` _mesh "/Game/HorseStarterKit/Animation/Dismount_Right_Rider.Dismount_Right_Rider" false)
      (if (`SkeletalMeshComponent.IsPlaying` _mesh) :!label _label
        (`KismetSystemLibrary.Delay` 0.2)
        (goto _label)
        (else
          (`Actor.K2_AddActorLocalRotation` _owingcharacter (`self.GetRiderRotator` (stale `self.ReceiveTick` DeltaSeconds)) false false)
          (`SkeletalMeshComponent.PlayAnimation` _mesh "/Game/Musume/Character/Animation/Rider/Dance/Anim_RiderDance_UE.Anim_RiderDance_UE" false))))))

(event `self.ReceiveTick`
  (params (DeltaSeconds :type "Float (single-precision)")))