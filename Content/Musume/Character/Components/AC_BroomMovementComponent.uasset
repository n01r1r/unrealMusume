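; Movement component for a ridden broom character that randomly halts mid-run to drop its rider and leave trash behind.
; Init and Movement defer to the parent component, while Tick adds a roughly one-in-a-thousand stop chance per frame while running.
; On a stop it zeroes speed, then after a delay detaches and grounds the rider, plays a dismount animation, attaches the broom to the rider and spawns BP_Trash in parallel.
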(event `self.ReceiveBeginPlay`)

(event `self.ReceiveTick`
  (params (DeltaSeconds :type "Float (single-precision)"))
  (bind _owingcharacter (`self.OwingCharacter`))
  (bind _returnvalue (`Actor.GetTransform` (`self.OwingCharacter`)))
  (bind _rootcomponent (`Actor.RootComponent` _owingcharacter))
  (bind (_returnvalue_x _returnvalue_y) (`KismetMathLibrary.BreakVector` (`SceneComponent.K2_GetComponentLocation` _rootcomponent)))
  (bind (_returnvalue_roll _returnvalue_pitch _returnvalue_yaw) (`KismetMathLibrary.BreakRotator` (`SceneComponent.K2_GetComponentRotation` _rootcomponent)))
  (if (and (`self.isRun`) (== (mod (`KismetMathLibrary.RandomInteger` 1000) 1000) 1))
    (`|ExecutionSequence`
      (:`then_0`
        ;[1 1 1] Stop Horse
        (`MovementComponent.StopMovementImmediately` (`self.CharacterMovementComponent`))
        (set `self.SpeedRandomValueRange` (0.0 0.0))
        (set `self.isRun` false)
        (`KismetSystemLibrary.Delay` 1.0)
        (bind _asrider_character (cast `RiderCharacter` (`|GetArrayItem` (`Actor.GetAttachedActors` _owingcharacter true false))))
        (bind _output_get (set `self.Rider` _asrider_character))
        (`Actor.K2_DetachFromActor` _asrider_character "KeepWorld" "KeepWorld" "KeepRelative")
        (`SceneComponent.K2_SetWorldLocationAndRotation` (`Actor.RootComponent` _output_get) (`KismetMathLibrary.MakeVector` _returnvalue_x _returnvalue_y -10.0) (`KismetMathLibrary.MakeRotator` 0.0 90.0 _returnvalue_yaw) false false)
        (`SkeletalMeshComponent.PlayAnimation` (`Character.Mesh` _output_get) "/Game/HorseStarterKit/Animation/Dismount_Right_Rider.Dismount_Right_Rider" false)
        (`Actor.K2_AttachToActor` (`self.OwingCharacter`) (`self.Rider`) "None" "KeepWorld" "KeepWorld" "KeepWorld" true))
      (:`then_1`
        ;[1 1 1] Spawn Trash
        (`KismetSystemLibrary.Delay` 1.0)
        (`|SpawnActorFromClass` "/Game/Musume/Character/BP_Trash.BP_Trash_C" (`KismetMathLibrary.MakeTransform` (`KismetMathLibrary.MakeVector` (.x (.location _returnvalue)) (.y (.location _returnvalue))) (.rotation _returnvalue) (.scale _returnvalue)) "AlwaysSpawn" "MultiplyWithRoot" null null)))))

(event `self.Init`
  (`parent.Init`))

(event `self.Movement`
  (params (DeltaTime :type "Float (single-precision)"))
  (`parent.Movement` DeltaTime))