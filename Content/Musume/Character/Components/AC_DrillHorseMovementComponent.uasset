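; Horse movement component variant for the drill horse, which knocks away horses it runs into.
; On BeginPlay the drill event calls an empty RollHead hook, scales the random speed range and binds the owner's capsule overlap.
; An overlapping horse character is launched along the owner's rotated forward vector, with the side picked by a cross-product left/right test.
; Init and Movement defer to the parent; debug prints remain.
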(event `self.ReceiveBeginPlay`
  (`|ExecutionSequence`
    (:`then_0`
      (`self.Active Drill Event`))))

(event `self.ReceiveTick`
  (params (DeltaSeconds :type "Float (single-precision)")))

(event `self.Init`
  (`parent.Init`))

(event `self.Movement`
  (params (DeltaTime :type "Float (single-precision)"))
  (`parent.Movement` DeltaTime))

(event `RollHead`)

(event `Active Drill Event`
  (bind _returnvalue (`self.GetOwner`))
  ;[1 1 1] 드릴 이벤트
  (`|ExecutionSequence`
    (:`then_0`
      (`self.RollHead`))
    (:`then_1`
      (set `self.SpeedRandomValueRange` (* (`self.SpeedRandomValueRange`) (1.1 1.0))))
    (:`then_2`
      (`/Engine/EditorBlueprintResources/StandardMacros.IsValid` _returnvalue
        (:`Is Valid`
          (bind _ashorse_character (cast `HorseCharacter` _returnvalue))
          (`/Engine/EditorBlueprintResources/StandardMacros.IsValid` _ashorse_character
            (:`Is Valid`
              (add `PrimitiveComponent.OnComponentBeginOverlap` (`Character.CapsuleComponent` _ashorse_character) (delegate `OnComponentBeginOverlap_이벤트`))
              (`KismetSystemLibrary.PrintString` "binded"))))))))

(event `OnComponentBeginOverlap_이벤트`
  (params (OverlappedComponent :type "PrimitiveComponent Object Reference") (OtherActor :type "Actor Object Reference") (OtherComp :type "PrimitiveComponent Object Reference") (OtherBodyIndex :type Integer) (bFromSweep :type Boolean) (SweepResult :type "HitResult Structure (by ref)"))
  ;[1 1 1] 드릴 이벤트
  (`KismetSystemLibrary.PrintString` (`KismetSystemLibrary.GetDisplayName` OtherActor))
  (`self.makeImpulse` OtherActor))