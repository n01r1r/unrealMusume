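; AC_DrillMovement is a movement component for a drill horse variant, extending the parent's init and movement.
; On init it sets the third mesh child to the drill anim class, applies a neutral speed-range multiplier and binds capsule overlap.
; Overlaps only print the other actor's name.
; An unconnected impulse function would launch other horses along an angled direction, chosen by a cross-product side test.
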(event `self.Init`
  (`parent.Init`)
  (`self.Active Drill Event`))

(event `self.Movement`
  (params (DeltaTime :type "Float (single-precision)"))
  (`parent.Movement` DeltaTime))

(event `RollHead`
  (bind _mesh (`Character.Mesh` (`self.OwingCharacter`)))
  (bind _returnvalue (`SceneComponent.GetChildComponent` _mesh 2))
  (`/Engine/EditorBlueprintResources/StandardMacros.IsValid` _mesh
    (:`Is Valid`
      (bind `_as스켈레탈_메시_컴포넌트` (cast `SkeletalMeshComponent` _returnvalue)
        (:`then`
          (`SkeletalMeshComponent.SetAnimInstanceClass` `_as스켈레탈_메시_컴포넌트` "/Game/Musume/Character/ABP_DrillHorse.ABP_DrillHorse_C")
          (`KismetSystemLibrary.PrintString` (`KismetSystemLibrary.GetDisplayName` _returnvalue)))
        (:`CastFailed`
          (`KismetSystemLibrary.PrintString` "failed"))))))

(event `Active Drill Event`
  (`|ExecutionSequence`
    (:`then_0`
      (`self.RollHead`))
    (:`then_1`
      (set `self.SpeedRandomValueRange` (* (`self.SpeedRandomValueRange`) (1.0 1.0))))
    (:`then_2`
      (add `PrimitiveComponent.OnComponentBeginOverlap` (`Character.CapsuleComponent` (`self.OwingCharacter`)) (delegate `OnComponentBeginOverlap`))
      (`KismetSystemLibrary.PrintString` "binded"))))

(event `OnComponentBeginOverlap`
  (params (OverlappedComponent :type "PrimitiveComponent Object Reference") (OtherActor :type "Actor Object Reference") (OtherComp :type "PrimitiveComponent Object Reference") (OtherBodyIndex :type Integer) (bFromSweep :type Boolean) (SweepResult :type "HitResult Structure (by ref)"))
  (`KismetSystemLibrary.PrintString` (`KismetSystemLibrary.GetDisplayName` OtherActor)))