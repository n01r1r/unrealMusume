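; Player spawner actor that creates a mounted horse and rider pair at its own transform when play begins.
; BeginPlay hides the Cube mesh, spawns the horse and passes it AC_HorseMovementComponent through AddACHorseMovementComponent.
; It then spawns the rider at a fixed offset, sets the horse as its riding target and attaches it.
; Finally, it copies the spawner's PlayerInfo into the rider's PlayerInfoUI widget.
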(event `self.ReceiveBeginPlay`
  (`SceneComponent.SetVisibility` (`self.Cube`) false false)
  (bind _returnvalue (`|SpawnActorFromClass` "/Game/Musume/Character/BP_HorseCharacter.BP_HorseCharacter_C" (`self.GetTransform`) "Undefined" "MultiplyWithRoot" null null))
  (`|AddComponentByClass` _returnvalue "/Game/Musume/Character/Components/AC_HorseMovementComponent.AC_HorseMovementComponent_C")
  (bind _returnvalue_2 (`|SpawnActorFromClass` "/Game/Musume/Character/BP_RiderCharacter.BP_RiderCharacter_C" (`KismetMathLibrary.MakeTransform` (- (.location (`self.GetTransform`)) (230.0 20.0 40.0)) (.rotation (`self.GetTransform`)) (.scale (`self.GetTransform`))) "Undefined" "MultiplyWithRoot" null null))
  (set `RiderCharacter.RidingTarget` _returnvalue _returnvalue_2)
  (`RiderCharacter.AttachRiderToHorse` _returnvalue_2)
  (bind _asplayer_info_ui (cast `/Game/Musume/UI/UI_Kanttabbiya/PlayerInfoUI` (`WidgetComponent.GetWidget` (`/Game/Musume/Character/BP_RiderCharacter.PlayerInfoWidget` _returnvalue_2))))
  (set `/Game/Musume/UI/UI_Kanttabbiya/PlayerInfoUI.PlayerInfo` (`self.PlayerInfo`) _asplayer_info_ui))

(fn `UserConstructionScript`)