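; Finish-line trigger for a horse race that records finish times and ends the race.
; A looping 0.01-second timer drives a minute, second and hundredths clock, though GetTimeAsFloat divides the hundredths by 1000.
; Any first overlap starts a retire countdown, and each overlapping HorseCharacter appends its time string to ResultList, without duplicate checks.
; After three seconds, Tick pauses the clock, copies results to MusmeGameInstance and opens the Result level.
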(event `UpdateTimerEvent`
  (`self.UpdatTime`))

(event `self.ReceiveBeginPlay`
  (bind _returnvalue (`KismetSystemLibrary.K2_SetTimerDelegate` (`|CreateDelegate` :!event `UpdateTimerEvent`) 0.01 true))
  (set `self.TimerHandle` _returnvalue))

(event `self.ReceiveActorBeginOverlap`
  (params (OtherActor :type "Actor Object Reference"))
  (bind _returnvalue (`self.GetTimeAsString`))
  (`|ExecutionSequence`
    (:`then_0`
      ;[1 1 1] 리타이어 시작
      (if (not (`self.isRetiring`))
        (set `self.isRetiring` true)
        (set `self.RetiringTime` (`self.GetTimeAsFloat`))))
    (:`then_1`
      ;[1 1 1] 결승선 통과 말/기록 확인 / 중복 이슈 있을 수 있음
      (`KismetSystemLibrary.PrintString` _returnvalue)
      (cast `HorseCharacter` OtherActor)
      (`KismetSystemLibrary.PrintString` "horse")
      (`KismetArrayLibrary.Array_Add` (`self.ResultList`) _returnvalue))))

(event `self.ReceiveTick`
  (params (DeltaSeconds :type "Float (single-precision)"))
  ;[1 1 1] Retire확인
  (if (`self.isRetiring`)
    (if (>= (- (`self.GetTimeAsFloat`) (`self.RetiringTime`)) 3.0)
      (`KismetSystemLibrary.K2_PauseTimerHandle` (`self.TimerHandle`))
      (`KismetSystemLibrary.PrintString` "Race Over")
      ;[1 1 1] 기록 저장/레벨 전환
      (set `self.isRetiring` false)
      (bind _asmusme_game_instance (cast `/Game/Musume/MusmeGameInstance` (`GameplayStatics.GetGameInstance`))
        (:`then`
          (set `/Game/Musume/MusmeGameInstance.Results` (`self.ResultList`) _asmusme_game_instance)
          (`GameplayStatics.OpenLevel` "Result"))
        (:`CastFailed`
          (`KismetSystemLibrary.PrintString` "Cast Fail"))))))

(fn `UserConstructionScript`)