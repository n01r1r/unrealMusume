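; Actor component that moves the result-screen camera to frame characters.
; On BeginPlay it caches the level's CameraActor, then eases its scene component to new targets with MoveComponentTo.
; ZoomCharacterEvent takes location and yaw from the given transform, while MoveNextCharacter makes a quicker move that sets only location.
; Both derive camera X and Z through GetCameraXY, which holds fixed back and up offsets; Y passes through unchanged.
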(event `self.ReceiveBeginPlay`
  (bind _returnvalue (`GameplayStatics.GetActorOfClass` "/Script/Engine.CameraActor"))
  (set `self.CameraActor` _returnvalue))

(event `Zoom Character Event`
  (params (NewParam :type "Transform Structure"))
  (bind (_newx _newz) (`self.GetCameraXY` (.x (.location NewParam)) (.z (.location NewParam))))
  (`KismetSystemLibrary.MoveComponentTo` (`CameraActor.SceneComponent` (`self.CameraActor`)) (`KismetMathLibrary.MakeVector` _newx (.y (.location NewParam)) _newz) (`KismetMathLibrary.MakeRotator` 0.0 0.0 (.yaw (.rotation NewParam))) false true 0.4))

(event `Move Next Character`
  (params (NewParam :type "Transform Structure"))
  (bind (_newx _newz) (`self.GetCameraXY` (.x (.location NewParam)) (.z (.location NewParam))))
  (`KismetSystemLibrary.MoveComponentTo` (`CameraActor.SceneComponent` (`self.CameraActor`)) (`KismetMathLibrary.MakeVector` _newx (.y (.location NewParam)) _newz) (struct) true true 0.2))